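; Lightning strike actor that plays a light flash and delayed thunder when it begins play.
; One point light blinks briefly, then a Flash timeline drives a second light's intensity.
; In parallel, the summed signed XYZ offset to the first Player actor, scaled down, sets the thunder delay, imitating sound travel time without true distance.
; That same value picks between the ThunderC and ThunderF sounds.
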(event `self.ReceiveBeginPlay`
  (bind _pointlight1 (`self.PointLight1`))
  (bind (_returnvalue_x _returnvalue_y _returnvalue_z) (`KismetMathLibrary.BreakVector` (- (`self.K2_GetActorLocation` (`self.Player`)) (`self.K2_GetActorLocation`))))
  (bind _returnvalue (/ (+ _returnvalue_x _returnvalue_y _returnvalue_z) 5000.0))
  (bind _outactors (`GameplayStatics.GetAllActorsOfClass` "/Game/Jordan/Blueprints/General/Player.Player_C"))
  (set `self.Player` (`|GetArrayItem` _outactors))
  (`|ExecutionSequence`
    (:`then_0`
      (`SceneComponent.SetVisibility` _pointlight1 true false)
      (`KismetSystemLibrary.Delay` 0.1)
      (`SceneComponent.SetVisibility` _pointlight1 false false)
      (bind (_direction _newtrack_0) (`Timeline|Flash` :!via `PlayFromStart`)
        (:`Update`
          (`LightComponent.SetIntensity` (`self.PointLight`) (* _newtrack_0 1000.0)))))
    (:`then_1`
      (`KismetSystemLibrary.Delay` _returnvalue)
      (if (>= _returnvalue 5.0)
        (`AudioComponent.Play` (`self.Thunder-C`) 0.0)
        (else
          (`AudioComponent.Play` (`self.Thunder-F`) 0.0))))))

(fn `UserConstructionScript`)