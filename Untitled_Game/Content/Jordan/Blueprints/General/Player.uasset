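; First-person player Blueprint with walking, stamina-limited sprinting, mouse look, manual blinking and a weather-cycle input.
; Movement axes set IsWalking and drain RunAmount while running; Tick regenerates it through a Delay, slower while walking, and stops sprinting when empty.
; Mouse Y rotates the camera directly, reversing input past ±75° pitch to limit it.
; Blink drives the UI widget found at BeginPlay; CameraBob is an empty stub and WeatherSys is never assigned here.
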(event `InputAxis|LR`
  (params (AxisValue :type "Float (single-precision)"))
  (bind _returnvalue (`self.GetActorRightVector`))
  ;[1 1 1] Movement with run
  (set `self.Is walking` (or (> AxisValue 0.1) (< AxisValue -0.1)))
  (if (`self.Running`)
    (`self.AddMovementInput` _returnvalue (* AxisValue 1.3))
    (bind _output_get (set `self.Run amount` (- (stale _output_get) 0.05) :!label _label))
    (else
      (`self.AddMovementInput` _returnvalue (/ AxisValue 1.2)))))

(event `self.ReceiveTick`
  (params (DeltaSeconds :type "Float (single-precision)"))
  ;[1 1 1] Run amount
  (`self.CameraBob`)
  (if (<= (`self.Run amount`) 0.1)
    (set `self.Running` false)
    (else
      (`KismetSystemLibrary.Delay` 0.05)
      (if (`self.Running`)
        _
        (elif (>= (stale _output_get) 100.0)
          _
          (elif (`self.Is walking`)
            (bind _output_get (set `self.Run amount` (+ (stale _output_get) 0.15)))
            (else
              (bind _output_get_2 (set `self.Run amount` (+ (stale _output_get_2) 0.2))))))))))

(event `InputAxis|FB`
  (params (AxisValue :type "Float (single-precision)"))
  (bind _returnvalue (`self.GetActorForwardVector`))
  ;[1 1 1] Movement with run
  (set `self.Is walking` (or (> AxisValue 0.1) (< AxisValue -0.1)))
  (if (`self.Running`)
    (`self.AddMovementInput` _returnvalue (* AxisValue 1.3))
    (goto _label)
    (else
      (`self.AddMovementInput` _returnvalue (/ AxisValue 1.2)))))

(event `InputAction|Run`
  (params (Key :type "Key Structure"))
  ;[1 1 1] Run check
  (:`Pressed`
    (if (and (`self.Is walking`) (> (`self.Run amount`) 0.1))
      (set `self.Running` true)
      (else
        (set `self.Running` false :!label _label_2))))
  (:`Released`
    (goto _label_2)))

(event `InputAxis|Mouse X`
  (params (AxisValue :type "Float (single-precision)"))
  ;[1 1 1] Movement with run
  (`self.AddControllerYawInput` AxisValue))

(event `self.ReceiveBeginPlay`
  (bind _foundwidgets (`WidgetBlueprintLibrary.GetAllWidgetsOfClass` "/Game/Jordan/UI/UI.UI_C" false))
  (set `self.UI` (`|GetArrayItem` _foundwidgets)))

(event `CameraBob`
  (if (`self.Is walking`)
    (if (`self.Running`)
      _)))

(event `InputAction|CycleWeather`
  (params (Key :type "Key Structure"))
  (:`Pressed`
    (`/Game/Jordan/Blueprints/General/WeatherSys.Cycleweather` (`self.Weather Sys`))))

(event `InputAxis|Mouse Y`
  (params (AxisValue :type "Float (single-precision)"))
  (bind (_returnvalue_roll _returnvalue_pitch) (`KismetMathLibrary.BreakRotator` (`SceneComponent.K2_GetComponentRotation` (`self.Camera`))))
  ;[1 1 1] Mouse Y
  (`|ExecutionSequence`
    (:`then_0`
      (if (and (<= AxisValue 0.0) (<= _returnvalue_pitch -75.0))
        (`SceneComponent.K2_AddRelativeRotation` (`self.Camera`) (`KismetMathLibrary.MakeRotator` 0.0 (* AxisValue -1.0)) false false :!label _label_3)
        (else
          (`SceneComponent.K2_AddRelativeRotation` (`self.Camera`) (`KismetMathLibrary.MakeRotator` 0.0 AxisValue) false false :!label _label_4))))
    (:`then_1`
      (if (and (>= AxisValue 0.0) (>= _returnvalue_pitch 75.0))
        (goto _label_3)
        (else
          (goto _label_4))))))

(event `InputAction|Blink`
  (params (Key :type "Key Structure"))
  (bind _ui (`self.UI`))
  (:`Pressed`
    (`/Game/Jordan/UI/UI.M-Blink_P` _ui)
    (set `/Game/Jordan/UI/UI.Manual blink` true _ui))
  (:`Released`
    (`/Game/Jordan/UI/UI.M-Blink-UP` _ui)
    (set `/Game/Jordan/UI/UI.Manual blink` false _ui)))

(fn `UserConstructionScript`)