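; Weather controller actor that switches between clear, rain, snow and thunderstorm effects, activating the storm effect on BeginPlay.
; Cycleweather, not called within this Blueprint, picks a state from a reseeded random stream and repeats every 10–20 seconds.
; Snow starts the first found Floor actor, while other states stop it.
; Tick derives a storm flag that lets a delayed, self-calling event spawn Thunder actors at random surrounding positions.
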(event `self.ReceiveBeginPlay`
  (bind _outactors (`GameplayStatics.GetAllActorsOfClass` "/Game/Jordan/Blueprints/General/Floor.Floor_C"))
  (set `self.Floors` (`|GetArrayItem` _outactors))
  (`ActorComponent.Activate` (`self.RainStorm`) false :!label _label)
  (`ActorComponent.Deactivate` (`self.Snow`))
  (`ActorComponent.Deactivate` (`self.Rain`))
  (`self.Start thunder`)
  (`/Game/Jordan/Blueprints/General/Floor.Stop` (`self.Floors`) :!label _label_2))

(event `Cycleweather`
  (bind _rainstorm (`self.RainStorm`))
  (bind _rain (`self.Rain`))
  (bind _snow (`self.Snow`))
  (bind _rand_int (`self.Random Int` 0 4 :!label _label_3)
    (:`Out`
      (bind _output_get (set `self.Cycle` _rand_int))
      (`|ExecutionSequence`
        (:`then_0`
          (if (== _output_get 0)
            (`ActorComponent.Deactivate` _rain)
            (`ActorComponent.Deactivate` _snow)
            (`ActorComponent.Deactivate` _rainstorm)
            (goto _label_2)
            (elif (== _output_get 1)
              (`ActorComponent.Activate` _rain false)
              (`ActorComponent.Deactivate` _snow)
              (`ActorComponent.Deactivate` _rainstorm)
              (goto _label_2)
              (elif (== _output_get 2)
                (`ActorComponent.Activate` _snow false)
                (`ActorComponent.Deactivate` _rain)
                (`ActorComponent.Deactivate` _rainstorm)
                (`/Game/Jordan/Blueprints/General/Floor.Start` (`self.Floors`))
                (elif (== _output_get 3)
                  (goto _label))))))
        (:`then_1`
          (`KismetSystemLibrary.Delay` (`KismetMathLibrary.RandomFloatInRange` 10.0 20.0))
          (goto _label_3))))))

(event `self.ReceiveTick`
  (params (DeltaSeconds :type "Float (single-precision)"))
  (set `self.Thunder storm` (== (`self.Cycle`) 3)))

(event `Start thunder`
  (bind (_returnvalue_x _returnvalue_y _returnvalue_z) (`KismetMathLibrary.BreakVector` (`self.K2_GetActorLocation`)))
  (bind _returnvalue (`KismetMathLibrary.RandomFloatInRange` -10000.0 10000.0))
  (`KismetSystemLibrary.Delay` (`KismetMathLibrary.RandomFloatInRange` 5.0 20.0))
  (if (`self.Thunder storm`)
    (`|SpawnActorFromClass` "/Game/Jordan/Blueprints/General/Thunder.Thunder_C" (`KismetMathLibrary.MakeTransform` (`KismetMathLibrary.MakeVector` (+ _returnvalue_x _returnvalue) (+ _returnvalue _returnvalue_y) _returnvalue_z) (`KismetMathLibrary.MakeRotator` 0.0 0.0 (`KismetMathLibrary.RandomFloatInRange` 0.0 360.0))) "AlwaysSpawn" "OverrideRootScale" null null)
    (`self.Start thunder`)))

(fn `UserConstructionScript`)