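; Floor actor that gradually changes the snow amount on its cube's material, driven by Start and Stop events.
; Start resets a DoOnce on Tick, which creates a dynamic snow-gather material instance with zero snow and a set UV scale, then triggers SnowFall after a delay.
; SnowFall and Stop each play their own timeline to animate the Snow Amount parameter.
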(event `self.ReceiveTick`
  (params (DeltaSeconds :type "Float (single-precision)"))
  (`/Engine/EditorBlueprintResources/StandardMacros.DoOnce` true :!label _label
    (:`Completed`
      (bind _returnvalue (`PrimitiveComponent.CreateDynamicMaterialInstance` (`self.Cube`) 0 "/Game/Jordan/Mats/SnowGatherMat.SnowGatherMat" "None"))
      (`MaterialInstanceDynamic.SetScalarParameterValue` _returnvalue "Snow Amount" 0.0)
      (`MaterialInstanceDynamic.SetScalarParameterValue` _returnvalue "UV Scale" 15.0) ; Put UV Scale here
      (`KismetSystemLibrary.Delay` 10.0)
      (`self.Snow Fall`))))

(event `Start`
  (goto _label :!via `Reset`))

(event `Stop`
  (bind (_direction _snowamount) (`Timeline|Timeline_1` :!via `PlayFromStart`)
    (:`Update`
      (`MaterialInstanceDynamic.SetScalarParameterValue` (stale `self.ReceiveTick` _returnvalue) "Snow Amount" _snowamount))))

(event `Snow Fall`
  (bind (_direction _snowamount) (`Timeline|Timeline_0` :!via `PlayFromStart`)
    (:`Update`
      (`MaterialInstanceDynamic.SetScalarParameterValue` (stale `self.ReceiveTick` _returnvalue) "Snow Amount" _snowamount))))

(fn `UserConstructionScript`)