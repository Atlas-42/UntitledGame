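; SCP-173 enemy actor that turns to face the player and lunges toward them while they are inside its Sphere.
; Each Tick it steps forward without sweep if not looked at, or if looked at while Activate is set, but never during a blink.
; Blinking from the game instance or leaving the Sphere clears Activate, and a DoOnce re-arms it after a short delay.
; Leaving also sets IdleAI, and Activate is debug-printed every frame.
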(event `self.ReceiveBeginPlay`
  (bind _asdata (cast `/Game/Jordan/Misc/Data` (`GameplayStatics.GetGameInstance`)))
  (set `self.Data` _asdata)
  (bind _outactors (`GameplayStatics.GetAllActorsOfClass` "/Game/Jordan/Blueprints/General/Player.Player_C"))
  (set `self.Player` (`|GetArrayItem` _outactors)))

(event `self.ReceiveTick`
  (params (DeltaSeconds :type "Float (single-precision)"))
  (bind _player (`self.Player`))
  (`KismetSystemLibrary.PrintString` (`KismetStringLibrary.Conv_BoolToString` (`self.Activate`)))
  (if (`PrimitiveComponent.IsOverlappingActor` (`self.Sphere`) _player)
    (set `self.Idle AI` false)
    (if (`/Game/Jordan/Misc/Data.Blinking` (`self.Data`))
      (set `self.Activate` false :!label _label)
      (goto _label_2 :!via `Reset`)
      (else
        (`|ExecutionSequence`
          (:`then_0`
            (`/Engine/EditorBlueprintResources/StandardMacros.DoOnce` false :!label _label_2
              (:`Completed`
                (`KismetSystemLibrary.Delay` 0.2)
                (bind _output_get (set `self.Activate` true)))))
          (:`then_1`
            (if (`self.Is Looking at`)
              (if _output_get
                (`self.K2_SetActorRelativeRotation` (`KismetMathLibrary.MakeRotator` 0.0 0.0 (.yaw (`KismetMathLibrary.FindLookAtRotation` (`self.K2_GetActorLocation`) (`self.K2_GetActorLocation` _player)))) :!label _label_3)
                (`self.K2_AddActorLocalOffset` (60.0 0.0 0.0)))
              (else
                (goto _label_3)))))))
    (else
      (set `self.Idle AI` true)
      (goto _label))))

(fn `UserConstructionScript`)