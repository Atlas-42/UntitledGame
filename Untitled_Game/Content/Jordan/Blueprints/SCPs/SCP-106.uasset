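; SCP-106 is an enemy actor that pursues the player while they overlap its Sphere component.
; It caches the first Player actor on BeginPlay, then each Tick yaws to the player-to-self direction and steps along negative local X, closing in on the player.
; Movement is unswept, so it passes through geometry, and uses a fixed per-frame offset, so speed depends on frame rate.
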(event `self.ReceiveBeginPlay`
  (bind _outactors (`GameplayStatics.GetAllActorsOfClass` "/Game/Jordan/Blueprints/General/Player.Player_C"))
  (set `self.Player` (`|GetArrayItem` _outactors)))

(event `self.ReceiveTick`
  (params (DeltaSeconds :type "Float (single-precision)"))
  (if (`PrimitiveComponent.IsOverlappingActor` (`self.Sphere`) (`self.Player`))
    (`self.K2_SetActorRelativeRotation` (`KismetMathLibrary.MakeRotator` 0.0 0.0 (.yaw (`KismetMathLibrary.FindLookAtRotation` (`self.K2_GetActorLocation` (`self.Player`)) (`self.K2_GetActorLocation`)))))
    (`self.K2_AddActorLocalOffset` (-4.2 0.0 0.0))))

(fn `UserConstructionScript`)